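; Playable card actor that the player hovers, drags from hand and drops onto the board, driven by widget mouse events and a Hand/Board state.
; Hovering doubles its scale, also offsetting it in Hand; pressing in Hand opens a Tick gate that teleports it under the cursor trace.
; Release passes it to the BoardCollisionCheck actor's DragCard, restores its original location and frees the hand tile.
; Random data-table stat setup in the construction script is disconnected.
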(event OnReleased(Widget)
  (params (TouchedComponent :type Primitive%20Component%20Object%20Reference) (ButtonReleased :type Key%20Structure :default "None"))
  (Development|PrintString "RELEASED")
  (switch Utilities|FlowControl|Switch|SwitchonCard_States (Variables|Default|GetCurrent%20State)
    (:NewEnumerator1
      (Utilities|FlowControl|Gate false
        (:Exit
          (Default|DragCard (Variables|Default|GetPlayerBoard) self)
          (Development|PrintString "Drag Card fv után")
          (Variables|Default|SetMouseRelased true)
          (CallFunction|CloseGate)
          (Transformation|Teleport (Variables|Default|GetOld%20Location) "0, 0, 0")
          (Variables|/Game/Blueprints/Board_Blueprints/HandTile.HandTile_C|SetisTileTaken (Variables|Default|GetPlayerHandTile) false))))))

(event OnBeginCursorOver(CardFront)
  (params (TouchedComponent :type Primitive%20Component%20Object%20Reference)))

(event OnEndCursorOver(CardFront)
  (params (TouchedComponent :type Primitive%20Component%20Object%20Reference)))

(event OnClicked(CardFront)
  (params (TouchedComponent :type Primitive%20Component%20Object%20Reference) (ButtonPressed :type Key%20Structure :default "None")))

(event OnClicked(Widget)
  (params (TouchedComponent :type Primitive%20Component%20Object%20Reference) (ButtonPressed :type Key%20Structure :default "None"))
  (bind _returnvalue (Game|GetPlayerController 0))
  (bind _hitresult (Game|Player|GetHitResultUnderCursorbyChannel _returnvalue "TraceTypeQuery1" true))
  (bind _location (Collision|BreakHitResult _hitresult))
  (bind (_x _y) (Math|Vector|BreakVector _location))
  (Development|PrintString "CLICKED")
  (switch Utilities|FlowControl|Switch|SwitchonCard_States (Variables|Default|GetCurrent%20State)
    (:NewEnumerator1
      (Variables|Default|SetOld%20Rot (Transformation|GetWorldRotation (Variables|Actor|GetDefaultSceneRoot)))
      (Utilities|FlowControl|Gate false
        (:Exit
          (Variables|Default|SetMouseRelased false)
          (Utilities|FlowControl|Gate true) ; enters at Open
        )))))

(event OnBeginCursorOver(Widget)
  (params (TouchedComponent :type Primitive%20Component%20Object%20Reference))
  (switch Utilities|FlowControl|Switch|SwitchonCard_States (Variables|Default|GetCurrent%20State)
    (:NewEnumerator1
      _)
    (:NewEnumerator2
      _))
  (CallFunction|OnHover))

(event OnEndCursorOver(Widget)
  (params (TouchedComponent :type Primitive%20Component%20Object%20Reference))
  (bind _returnvalue (Game|GetPlayerController 0))
  (switch Utilities|FlowControl|Switch|SwitchonCard_States (Variables|Default|GetCurrent%20State)
    (:NewEnumerator1
      _)
    (:NewEnumerator2
      _))
  (CallFunction|EndHover)
  (Variables|/Script/Engine.PlayerController|SetbEnableMouseOverEvents _returnvalue false)
  (Utilities|FlowControl|Delay 0.2)
  (Variables|/Script/Engine.PlayerController|SetbEnableMouseOverEvents _returnvalue true))

(event OnReleased(CardFront)
  (params (TouchedComponent :type Primitive%20Component%20Object%20Reference) (ButtonReleased :type Key%20Structure :default "None")))

(event Custom|CloseGate
  (bind _returnvalue (Game|GetPlayerController 0))
  (bind _hitresult (Game|Player|GetHitResultUnderCursorbyChannel _returnvalue "TraceTypeQuery1" true))
  (bind _location (Collision|BreakHitResult _hitresult))
  (bind (_x _y) (Math|Vector|BreakVector _location))
  (Utilities|FlowControl|Gate true) ; enters at Close
)

(event Custom|CloseOnClickGate
  (bind _returnvalue (Game|GetPlayerController 0))
  (bind _hitresult (Game|Player|GetHitResultUnderCursorbyChannel _returnvalue "TraceTypeQuery1" true))
  (bind _location (Collision|BreakHitResult _hitresult))
  (bind (_x _y) (Math|Vector|BreakVector _location))
  (Utilities|FlowControl|Gate false) ; enters at Close
)

(event EventTick
  (params (DeltaSeconds :type Float%20%28single-precision%29))
  (bind _returnvalue (Game|GetPlayerController 0))
  (bind _hitresult (Game|Player|GetHitResultUnderCursorbyChannel _returnvalue "TraceTypeQuery1" true))
  (bind _location (Collision|BreakHitResult _hitresult))
  (bind (_x _y) (Math|Vector|BreakVector _location))
  (Utilities|FlowControl|Gate true
    (:Exit
      (Transformation|Teleport (Math|Vector|MakeVector (+ _x 3e+01) _y (.Z (Math|Vector|BreakVector (Transformation|GetActorLocation)))) "0, 0, 0"))))

(event EventBeginPlay
  (bind _defaultsceneroot (Variables|Actor|GetDefaultSceneRoot))
  (Variables|Default|SetOld%20Location (Transformation|GetWorldLocation _defaultsceneroot))
  (Variables|Default|SetOld%20Scale (Transformation|GetWorldScale _defaultsceneroot))
  (bind _outactors (Actor|GetAllActorsOfClass "/Game/Blueprints/Board_Blueprints/BoardCollisionCheck.BoardCollisionCheck_C"))
  (Variables|Default|SetPlayerBoard (Utilities|Array|Get(acopy) _outactors)))

(fn ConstructionScript)

(fn OnHover
  (Development|PrintString "HOVER BEGIN")
  (switch Utilities|FlowControl|Switch|SwitchonCard_States (Variables|Default|GetCurrent%20State)
    (:NewEnumerator1
      (Transformation|Teleport (+ (Variables|Default|GetOld%20Location) (Variables|Default|GetHover%20Offset)) (Transformation|GetActorRotation)))
    (:NewEnumerator2
      _))
  (Transformation|SetWorldScale3D (Variables|Actor|GetDefaultSceneRoot) (* (Variables|Default|GetOld%20Scale) 2.0)))

(fn EndHover
  (Development|PrintString "HOVER END")
  (switch Utilities|FlowControl|Switch|SwitchonCard_States (Variables|Default|GetCurrent%20State)
    (:NewEnumerator1
      (Transformation|Teleport (Variables|Default|GetOld%20Location) (Transformation|GetActorRotation)))
    (:NewEnumerator2
      _))
  (Transformation|SetWorldScale3D (Variables|Actor|GetDefaultSceneRoot) (Variables|Default|GetOld%20Scale)))

(fn UpdateValues)