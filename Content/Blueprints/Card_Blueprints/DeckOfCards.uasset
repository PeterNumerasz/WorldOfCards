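; Deck of cards Blueprint for a card game, meant to build cards from a data table, though still unfinished.
; ConstructDeck loops over every Card_DataTable row and reads it, but does not yet pass the data on.
; CreateBasicCard writes name, ability text and stats to the BasicCard's values and text displays.
; CreateSpellCard and CreateMythicCard are empty stubs.
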(event Custom|Construct%20Deck
  (bind _outrownames (DataTable|GetDataTableRowNames "/Game/Cards/Card_DataTable.Card_DataTable"))
  (for _array_element _outrownames
    (bind _returnvalue (Utilities|GetDataTableRow "/Game/Cards/Card_DataTable.Card_DataTable" _array_element))))

(fn ConstructionScript)

(fn CreateSpellCard
  (params (Card%20Name :type Text) (Card%20Ability%20Name :type Text) (Card%20Ability%20Desc :type Text)))

(fn CreateMythicCard)

(fn CreateBasicCard
  (params (Card%20Name :type Text) (Card%20Ability%20Name :type Text) (Card%20Ability%20Desc :type Text) (Card%20Power :type Integer) (Card%20Attack :type Integer) (Card%20Health :type Integer) (Card%20Haste :type Integer))
  (bind _basic_card (Variables|Default|GetBasic%20Card))
  (bind _basic_card_2 (Variables|Default|GetBasic%20Card))
  (bind _basic_card_3 (Variables|Default|GetBasic%20Card))
  (bind _basic_card_4 (Variables|Default|GetBasic%20Card))
  (bind _basic_card_5 (Variables|Default|GetBasic%20Card))
  (bind _basic_card_6 (Variables|Default|GetBasic%20Card))
  (bind _basic_card_7 (Variables|Default|GetBasic%20Card))
  (bind _output_get (Variables|/Game/Blueprints/Card_Blueprints/NormalCard.NormalCard_C|SetCard%20Name%20Value _basic_card Card%20Name))
  (Rendering|Components|TextRender|SetText (Variables|/Game/Blueprints/Card_Blueprints/NormalCard.NormalCard_C|GetCardName _basic_card) _output_get)
  (bind _output_get_2 (Variables|/Game/Blueprints/Card_Blueprints/NormalCard.NormalCard_C|SetCard%20Ability%20Description%20Value _basic_card_2 Card%20Ability%20Name))
  (Rendering|Components|TextRender|SetText (Variables|/Game/Blueprints/Card_Blueprints/NormalCard.NormalCard_C|GetDescription _basic_card_2) _output_get_2)
  (bind _output_get_3 (Variables|/Game/Blueprints/Card_Blueprints/NormalCard.NormalCard_C|SetCard%20Ability%20Description%20Value%201 _basic_card_3 Card%20Ability%20Desc))
  (Rendering|Components|TextRender|SetText (Variables|/Game/Blueprints/Card_Blueprints/NormalCard.NormalCard_C|GetDescription1 _basic_card_3) _output_get_3)
  (bind _output_get_4 (Variables|/Game/Blueprints/Card_Blueprints/NormalCard.NormalCard_C|SetCard%20Power%20Value _basic_card_7 Card%20Power))
  (Rendering|Components|TextRender|SetText (Variables|/Game/Blueprints/Card_Blueprints/NormalCard.NormalCard_C|GetPower _basic_card_7) (Utilities|Text|ToText(Integer) _output_get_4))
  (bind _output_get_5 (Variables|/Game/Blueprints/Card_Blueprints/NormalCard.NormalCard_C|SetCard%20Attack%20Value _basic_card_5 Card%20Attack))
  (Rendering|Components|TextRender|SetText (Variables|/Game/Blueprints/Card_Blueprints/NormalCard.NormalCard_C|GetAttack _basic_card_5) (Utilities|Text|ToText(Integer) _output_get_5))
  (bind _output_get_6 (Variables|/Game/Blueprints/Card_Blueprints/NormalCard.NormalCard_C|SetCard%20Health%20Value _basic_card_6 Card%20Health))
  (Rendering|Components|TextRender|SetText (Variables|/Game/Blueprints/Card_Blueprints/NormalCard.NormalCard_C|GetHealth _basic_card_6) (Utilities|Text|ToText(Integer) _output_get_6))
  (bind _output_get_7 (Variables|/Game/Blueprints/Card_Blueprints/NormalCard.NormalCard_C|SetCard%20Haste%20Value _basic_card_4 Card%20Haste))
  (Rendering|Components|TextRender|SetText (Variables|/Game/Blueprints/Card_Blueprints/NormalCard.NormalCard_C|GetHaste _basic_card_4) (Utilities|Text|ToText(Integer) _output_get_7)))