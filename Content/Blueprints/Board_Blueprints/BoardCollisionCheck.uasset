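; Board manager that snaps a card passed to DragCard onto an untaken board tile.
; BeginPlay gathers all BoardTile actors and sorts them by PlayerIndex into two player board variables.
; DragCard opens a Tick gate that searches all tiles, regardless of player or overlap, for a free one.
; It marks that tile taken, moves the card there, updates its state and tile reference, and DragCardOver closes the gate.
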(event Custom|Drag%20Card
  (params (Card%20ref :type Normal%20Card%20Object%20Reference))
  (Development|PrintString "Drag card fv-ben")
  (Utilities|FlowControl|Gate true) ; enters at Open
)

(event Custom|Drag%20Card%20Over
  (Utilities|FlowControl|Gate true) ; enters at Close
)

(event Custom|Break
  (bind _card (Variables|Default|GetCard))
  (Utilities|Array|ForEachLoopwithBreak (Variables|Default|GetTiles)) ; enters at Break
)

(event EventBeginPlay
  (Utilities|FlowControl|Sequence
    (:then_1
      (bind _outactors (Actor|GetAllActorsOfClass "/Game/Blueprints/Board_Blueprints/BoardTile.BoardTile_C"))
      (bind _output_get (Variables|Default|SetTiles _outactors))
      (for _array_element _output_get
        (if (== (Variables|/Game/Blueprints/Board_Blueprints/BoardTile.BoardTile_C|GetPlayerIndex _array_element) 0)
          (Variables|Default|SetPlayer1%20Board (Utilities|Array|MakeArray _array_element))
          (else
            (Variables|Default|SetPlayer2%20Board (Utilities|Array|MakeArray _array_element))))))))

(event EventTick
  (params (DeltaSeconds :type Float%20%28single-precision%29))
  (Utilities|FlowControl|Gate true
    (:Exit
      (bind _output_get (Variables|Default|SetCard (stale Custom|Drag%20Card Card%20ref)))
      (bind _array_index (Utilities|Array|ForEachLoopwithBreak (Variables|Default|GetTiles))
        (:LoopBody
          (if (not (Variables|/Game/Blueprints/Board_Blueprints/BoardTile.BoardTile_C|GetIsTileTaken (Utilities|Array|Get(acopy) (Variables|Default|GetTiles) _array_index)))
            (Utilities|FlowControl|Sequence
              (:then_0
                (CallFunction|Break))
              (:then_1
                (Variables|/Game/Blueprints/Board_Blueprints/BoardTile.BoardTile_C|SetIsTileTaken (Utilities|Array|Get(acopy) (Variables|Default|GetTiles) _array_index) true)
                (Transformation|SetActorTransform (Variables|Default|GetCard) (Math|Transform|MakeTransform (Transformation|GetActorLocation (Utilities|Array|Get(acopy) (Variables|Default|GetTiles) _array_index)) "0, 0, 0" (Variables|/Game/Blueprints/NormalCard.NormalCard_C|GetOld%20Scale (Variables|Default|GetCard))))
                (Variables|/Game/Blueprints/NormalCard.NormalCard_C|SetCurrent%20State (Variables|Default|GetCard) "NewEnumerator2")
                (CallFunction|DragCardOver))
              (:then_2
                (Variables|/Game/Blueprints/NormalCard.NormalCard_C|SetBoard%20Tile (Variables|Default|GetCard) (Utilities|Array|Get(acopy) (Variables|Default|GetTiles) _array_index))))))))))

(fn ConstructionScript)