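; NormalCard is a card actor that reacts to the mouse cursor hovering over it.
; The Card component's mouse-over event assigns an OnBeginCursorOver binding to OnMouseOverCard, then calls OnHover.
; OnHover teleports the actor to CardFront's world location plus HoverOffset, keeping its rotation, and sets the root's world scale to a fixed value.
; No logic here restores the position or scale when hovering ends.
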(event Custom|On%20Mouse%20Over%20%28Card%29
  (params (TouchedActor :type Actor%20Object%20Reference))
  (EventDispatchers|AssignOnBeginCursorOver (delegate Custom|On%20Mouse%20Over%20%28Card%29))
  (CallFunction|OnHover))

(event EventBeginPlay)

(event Collision|EventActorBeginOverlap
  (params (OtherActor :type Actor%20Object%20Reference)))

(event EventTick
  (params (DeltaSeconds :type Float%20%28single-precision%29)))

(fn ConstructionScript)

(fn OnHover
  (Transformation|Teleport (+ (Transformation|GetWorldLocation (Variables|Default|GetCardFront)) (Variables|Default|GetHover%20Offset)) (Transformation|GetActorRotation))
  (Transformation|SetWorldScale3D (Variables|Default|GetDefaultSceneRoot) "0.400000,0.400000,0.400000"))