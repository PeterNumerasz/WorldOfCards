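; BoardTile is a card-game board slot with a Box trigger, meant to take a card dropped onto it.
; Its placement chain checks and clears the NormalCard's mouse-release flag, sets owner and occupancy, then snaps the card to the box.
; Zone Check rotates and shrinks the overlapped card, ignoring its inputs.
; The chain is disconnected: Tick and overlap events are empty, so placement never runs.
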(event OnComponentBeginOverlap(Box)
  (params (OverlappedComponent :type Primitive%20Component%20Object%20Reference) (OtherActor :type Actor%20Object%20Reference) (OtherComp :type Primitive%20Component%20Object%20Reference) (OtherBodyIndex :type Integer) (bFromSweep :type Boolean) (SweepResult :type Hit%20Result%20Structure%20%28by%20ref%29)))

(event OnComponentEndOverlap(Box)
  (params (OverlappedComponent :type Primitive%20Component%20Object%20Reference) (OtherActor :type Actor%20Object%20Reference) (OtherComp :type Primitive%20Component%20Object%20Reference) (OtherBodyIndex :type Integer)))

(event EventTick
  (params (DeltaSeconds :type Float%20%28single-precision%29)))

(fn ConstructionScript)

(fn ZoneCheck
  (params (Card :type Normal%20Card%20Object%20Reference) (Zone%20Location :type Vector))
  (Transformation|SetActorTransform (Utilities|Array|Get(acopy) (Variables|Components|GetCardOverlapped)) (Math|Transform|MakeTransform "0, 0, 0" "0.000000,0.000000,-90.000000" "0.600000,0.600000,0.600000")))